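; Game mode for a Pang-style bubble shooter that runs the level countdown, win and loss checks, and drop-in second player.
; Looping timers tick the clock and poll remaining bubbles, ending the level with competitive or classic widget animations; death handling also branches on mode.
; It pushes lives, weapon and timeline-animated scores to the in-game HUD widget, keeps player state in the game instance, and handles restart and quit keys.
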(event `self.ReceiveBeginPlay`
  ;[1 1 1] Set the update time funtion to be checked every sec and enable the input
  (`KismetSystemLibrary.K2_SetTimer` null "UpdateTime" 1.0 true)
  (`self.EnableInput` (`GameplayStatics.GetPlayerController` 0))
  (`KismetSystemLibrary.K2_SetTimer` null "CheckBubblesDestroyed" 0.5 true))

(event `Key|R` :paused true
  (params (Key :type "Key Structure"))
  ;[1 1 1] In game controls
  ;;[1 1 1] If end level press r to restart
  (:`Pressed`
    (if (`self.IsEndLevel`)
      (`GameplayStatics.OpenLevel` "LevelOneMap")
      (bind _aspang_game_instance_bp (cast `/Game/PangBP/Blueprints/GameMode/PangGameInstance_BP` (`GameplayStatics.GetGameInstance`)))
      (set `/Game/PangBP/Blueprints/GameMode/PangGameInstance_BP.ScoreP1` 0.0 _aspang_game_instance_bp)
      (set `/Game/PangBP/Blueprints/GameMode/PangGameInstance_BP.ScoreP2` 0.0 _aspang_game_instance_bp)
      (if (`/Game/PangBP/Blueprints/GameMode/PangGameInstance_BP.Competitive?` _aspang_game_instance_bp)
        ;;[1 1 1] If competitive, 3 lifes
        (set `/Game/PangBP/Blueprints/GameMode/PangGameInstance_BP.PH2Left` 3 _aspang_game_instance_bp)
        (set `/Game/PangBP/Blueprints/GameMode/PangGameInstance_BP.PH1Left` 3 _aspang_game_instance_bp)
        (else
          ;;[1 1 1] if classic, just one life
          (set `/Game/PangBP/Blueprints/GameMode/PangGameInstance_BP.PH2Left` 1 _aspang_game_instance_bp)
          (set `/Game/PangBP/Blueprints/GameMode/PangGameInstance_BP.PH1Left` 1 _aspang_game_instance_bp))))))

(event `Key|Q` :paused true
  (params (Key :type "Key Structure"))
  ;[1 1 1] In game controls
  ;;[1 1 1] If end level press q to quit
  (:`Pressed`
    (if (`self.IsEndLevel`)
      (`GameplayStatics.OpenLevel` "MainMenuMap"))))

(event `Key|G`
  (params (Key :type "Key Structure"))
  ;[1 1 1] In game controls
  ;;[1 1 1] Spawn player 2 when pressed g
  (:`Pressed`
    (if (not (`self.PlayerSpawned`))
      (set `self.PlayerSpawned` true)
      (bind _charactercreated (`self.SpawnPlayer2`))
      (`self.ShowP2UI`)
      (`/Game/PangBP/Blueprints/PangCharacter_BP.SetPostHitInvencibility` _charactercreated))))

(event `ScoreAnimation`
  (params (ScoreToAdd :type "Float (double-precision)") (PlayerNum :type Integer))
  ;[1 1 1] Score animation, implemented in an event because timelines cant be used infunctions
  (bind _aspang_game_instance_bp (cast `/Game/PangBP/Blueprints/GameMode/PangGameInstance_BP` (`GameplayStatics.GetGameInstance`)))
  (switch `int` PlayerNum
    (:`Default`
      (bind (_direction _alphatrack) (`Timeline|Timeline_0` :!via `PlayFromStart` :!label _label)
        (:`Update`
          (bind _scorep1 (`/Game/PangBP/Blueprints/GameMode/PangGameInstance_BP.ScoreP1` _aspang_game_instance_bp))
          (bind _returnvalue (+ _scorep1 ScoreToAdd))
          (`self.AddScore` (`KismetMathLibrary.Lerp` _scorep1 _returnvalue _alphatrack) PlayerNum))
        (:`Finished`
          (set `/Game/PangBP/Blueprints/GameMode/PangGameInstance_BP.ScoreP1` _returnvalue _aspang_game_instance_bp))))
    (:`0`
      (goto _label :!via `PlayFromStart`))
    (:`1`
      (bind (_direction_2 _alphatrack_2) (`Timeline|Timeline_1` :!via `PlayFromStart`)
        (:`Update`
          (bind _scorep2 (`/Game/PangBP/Blueprints/GameMode/PangGameInstance_BP.ScoreP2` _aspang_game_instance_bp))
          (bind _returnvalue_2 (+ _scorep2 ScoreToAdd))
          (`self.AddScore` (`KismetMathLibrary.Lerp` _scorep2 _returnvalue_2 _alphatrack_2) PlayerNum))
        (:`Finished`
          (set `/Game/PangBP/Blueprints/GameMode/PangGameInstance_BP.ScoreP2` _returnvalue_2 _aspang_game_instance_bp))))))

(fn `AddScore`
  (params (ScoreToShow :type "Float (double-precision)") (PlayerNum :type Integer))
  (bind _aspang_hud (cast `/Game/PangBP/Blueprints/GameMode/PangHUD` (`PlayerController.GetHUD` (`GameplayStatics.GetPlayerController` 0)))
    (:`then`
      (bind _asin__game_widget (cast `/Game/PangBP/Blueprints/UI/In-GameWidget` (`/Game/PangBP/Blueprints/GameMode/PangHUD.CurrentWidget` _aspang_hud)))
      ;[1 1 1] For player 1 or 2?
      (switch `int` PlayerNum
        (:`Default`
          ;[1 1 1] Add score to P1
          (`TextBlock.SetText` (`/Game/PangBP/Blueprints/UI/In-GameWidget.ScoreNumber` _asin__game_widget) (`|FormatText` "{Value}" (`KismetMathLibrary.Round` ScoreToShow)) :!label _label))
        (:`0`
          (goto _label))
        (:`1`
          ;[1 1 1] Add score to P2
          (`TextBlock.SetText` (`/Game/PangBP/Blueprints/UI/In-GameWidget.ScoreNumber2` _asin__game_widget) (`|FormatText` "{Value}" (`KismetMathLibrary.Round` ScoreToShow))))))
    (:`CastFailed`
      (`KismetSystemLibrary.PrintString` "Wrong HUD, change to PangHUD"))))

(fn `ChangePlayerWeaponUI`
  (params (PlayerNumber :type Integer) (WeaponNumber :type Integer))
  (bind _aspang_hud (cast `/Game/PangBP/Blueprints/GameMode/PangHUD` (`PlayerController.GetHUD` (`GameplayStatics.GetPlayerController` 0)))
    (:`then`
      (bind _asin__game_widget (cast `/Game/PangBP/Blueprints/UI/In-GameWidget` (`/Game/PangBP/Blueprints/GameMode/PangHUD.CurrentWidget` _aspang_hud)))
      ;[1 1 1] For player 1 or 2?
      (switch `int` PlayerNumber
        (:`0`
          ;[1 1 1] Set weapon image and text for player 1 UI
          (switch `int` WeaponNumber
            (:`Default`
              (bind _weaponimage (`/Game/PangBP/Blueprints/UI/In-GameWidget.WeaponImage` _asin__game_widget))
              (`Image.SetBrushFromTexture` _weaponimage "/Game/Pang/UIAssets/NormalHarpoon.NormalHarpoon" false :!label _label)
              (bind _weapontext (`/Game/PangBP/Blueprints/UI/In-GameWidget.WeaponText` _asin__game_widget))
              (`TextBlock.SetText` _weapontext "Hook"))
            (:`0`
              (goto _label))
            (:`1`
              (`Image.SetBrushFromTexture` _weaponimage "/Game/Pang/UIAssets/GrabHook.GrabHook" false)
              (`TextBlock.SetText` _weapontext "Grab Hook"))
            (:`2`
              (`Image.SetBrushFromTexture` _weaponimage "/Game/Pang/UIAssets/DoubleHook.DoubleHook" false)
              (`TextBlock.SetText` _weapontext "Double Hook"))
            (:`3`
              (`Image.SetBrushFromTexture` _weaponimage "/Game/Pang/UIAssets/gun.gun" false)
              (`TextBlock.SetText` _weapontext "Gun"))
            (:`4`
              (`Image.SetBrushFromTexture` _weaponimage "/Game/Pang/UIAssets/bubble.bubble" false)
              (`TextBlock.SetText` _weapontext "Bubble Gun"))))
        (:`1`
          ;[1 1 1] Set weapon image and text for player 2 UI
          (switch `int` WeaponNumber
            (:`Default`
              (bind _weaponimage2 (`/Game/PangBP/Blueprints/UI/In-GameWidget.WeaponImage2` _asin__game_widget))
              (`Image.SetBrushFromTexture` _weaponimage2 "/Game/Pang/UIAssets/NormalHarpoon.NormalHarpoon" false :!label _label_2)
              (bind _weapontext2 (`/Game/PangBP/Blueprints/UI/In-GameWidget.WeaponText2` _asin__game_widget))
              (`TextBlock.SetText` _weapontext2 "Hook"))
            (:`0`
              (goto _label_2))
            (:`1`
              (`Image.SetBrushFromTexture` _weaponimage2 "/Game/Pang/UIAssets/GrabHook.GrabHook" false)
              (`TextBlock.SetText` _weapontext2 "Grab Hook"))
            (:`2`
              (`Image.SetBrushFromTexture` _weaponimage2 "/Game/Pang/UIAssets/DoubleHook.DoubleHook" false)
              (`TextBlock.SetText` _weapontext2 "Double Hook"))
            (:`3`
              (`Image.SetBrushFromTexture` _weaponimage2 "/Game/Pang/UIAssets/gun.gun" false)
              (`TextBlock.SetText` _weapontext2 "Gun"))
            (:`4`
              (`Image.SetBrushFromTexture` _weaponimage2 "/Game/Pang/UIAssets/bubble.bubble" false)
              (`TextBlock.SetText` _weapontext2 "Bubble Gun"))))))
    (:`CastFailed`
      (`KismetSystemLibrary.PrintString` "Wrong HUD, change to PangHUD"))))

(fn `CheckBubblesDestroyed`
  ;[1 1 1] Check number of bubbles and if == 0, then trigger the level finished event and animation
  (if (`self.IsPlaying`)
    (if (<= (`self.NumberOfBubbles`) 0)
      (`KismetSystemLibrary.PrintString` "End game for bubbles")
      (bind _aspang_hud (cast `/Game/PangBP/Blueprints/GameMode/PangHUD` (`PlayerController.GetHUD` (`GameplayStatics.GetPlayerController` 0))))
      (bind _asin__game_widget (cast `/Game/PangBP/Blueprints/UI/In-GameWidget` (`/Game/PangBP/Blueprints/GameMode/PangHUD.CurrentWidget` _aspang_hud)))
      (set `self.IsEndLevel` true)
      ;;[1 1 1] trigger the appropiate event when no bubbles are left
      (bind _aspang_game_instance_bp (cast `/Game/PangBP/Blueprints/GameMode/PangGameInstance_BP` (`GameplayStatics.GetGameInstance`)))
      (if (`/Game/PangBP/Blueprints/GameMode/PangGameInstance_BP.Competitive?` _aspang_game_instance_bp)
        (`/Game/PangBP/Blueprints/UI/In-GameWidget.CompetitiveEndAnim` _asin__game_widget)
        (else
          (`/Game/PangBP/Blueprints/UI/In-GameWidget.LevelCompletedAnim` _asin__game_widget))))))

(fn `CheckDeath`
  (params (DeadPlayer :type "/Game/PangBP/Blueprints/PangCharacter_BP Object Reference"))
  (bind _aspang_game_instance_bp (cast `/Game/PangBP/Blueprints/GameMode/PangGameInstance_BP` (`GameplayStatics.GetGameInstance`)))
  (`/Engine/EditorBlueprintResources/StandardMacros.IncrementInt` (`self.DeadPlayers`)
    (:`  `
      (if (`/Game/PangBP/Blueprints/GameMode/PangGameInstance_BP.TwoPlayers?` _aspang_game_instance_bp)
        ;[1 1 1] Check if competitive game mode
        (if (`/Game/PangBP/Blueprints/GameMode/PangGameInstance_BP.Competitive?` _aspang_game_instance_bp)
          ;[1 1 1] If it's competitive game mode...
          ;;[1 1 1] Hide actor for 4 seconds and then revive
          (`/Game/PangBP/Blueprints/PangCharacter_BP.DisableCharacterTemporarily` DeadPlayer (`/Game/PangBP/Blueprints/PangCharacter_BP.PlayerID` DeadPlayer))
          (else
            ;[1 1 1] If multiplayer classic mode...
            ;;[1 1 1] If both players dead, end game
            (if (< (`self.DeadPlayers`) 2)
              (`self.SetActorHiddenInGame` DeadPlayer true)
              (set `/Game/PangBP/Blueprints/PangCharacter_BP.IsDisabled?` true DeadPlayer)
              (else
                ;[1 1 1] If only classic, single player, just restart the level
                (bind _aspang_hud (cast `/Game/PangBP/Blueprints/GameMode/PangHUD` (`PlayerController.GetHUD` (`GameplayStatics.GetPlayerController` 0)) :!label _label))
                (bind _asin__game_widget (cast `/Game/PangBP/Blueprints/UI/In-GameWidget` (`/Game/PangBP/Blueprints/GameMode/PangHUD.CurrentWidget` _aspang_hud)))
                (`/Game/PangBP/Blueprints/UI/In-GameWidget.GameOverAnim` _asin__game_widget)
                (set `self.IsEndLevel` true)))))
        (else
          (goto _label))))))

(fn `SetTime`
  (bind _aspang_hud (cast `/Game/PangBP/Blueprints/GameMode/PangHUD` (`PlayerController.GetHUD` (`GameplayStatics.GetPlayerController` 0)))
    (:`then`
      (bind _asin__game_widget (cast `/Game/PangBP/Blueprints/UI/In-GameWidget` (`/Game/PangBP/Blueprints/GameMode/PangHUD.CurrentWidget` _aspang_hud)))
      (`TextBlock.SetText` (`/Game/PangBP/Blueprints/UI/In-GameWidget.TimeNumber` _asin__game_widget) (`|FormatText` "{Value}" (`self.TimeLeft`))))
    (:`CastFailed`
      (`KismetSystemLibrary.PrintString` "Wrong HUD, change to PangHUD"))))

(fn `ShowP2UI`
  (bind _aspang_hud (cast `/Game/PangBP/Blueprints/GameMode/PangHUD` (`PlayerController.GetHUD` (`GameplayStatics.GetPlayerController` 0)))
    (:`then`
      (bind _asin__game_widget (cast `/Game/PangBP/Blueprints/UI/In-GameWidget` (`/Game/PangBP/Blueprints/GameMode/PangHUD.CurrentWidget` _aspang_hud)))
      (`Widget.SetVisibility` (`/Game/PangBP/Blueprints/UI/In-GameWidget.JoinP2` _asin__game_widget) "Hidden")
      (`Widget.SetVisibility` (`/Game/PangBP/Blueprints/UI/In-GameWidget.Player2CoverImage` _asin__game_widget) "Hidden"))
    (:`CastFailed`
      (`KismetSystemLibrary.PrintString` "Wrong HUD, change to PangHUD"))))

(fn `SpawnPlayer2`
  (returns (CharacterCreated :type "/Game/PangBP/Blueprints/PangCharacter_BP Object Reference"))
  ;[1 1 1] Spawn the player 2
  (`GameplayStatics.CreatePlayer` 1)
  (bind _returnvalue (`|SpawnActorFromClass` "/Game/PangBP/Blueprints/PangCharacter_BP.PangCharacter_BP_C" (`KismetMathLibrary.MakeTransform` (1200.0 580.0 250.0)) "AlwaysSpawn" "OverrideRootScale" null null))
  (set `/Game/PangBP/Blueprints/PangCharacter_BP.PlayerID` 1 _returnvalue)
  (`Controller.Possess` (`GameplayStatics.GetPlayerController` 1) _returnvalue)
  (bind _aspang_game_instance_bp (cast `/Game/PangBP/Blueprints/GameMode/PangGameInstance_BP` (`GameplayStatics.GetGameInstance`)))
  (set `/Game/PangBP/Blueprints/GameMode/PangGameInstance_BP.TwoPlayers?` true _aspang_game_instance_bp)
  (`self.UpdateHP` 1)
  (set `self.PlayerSpawned` true)
  (return _returnvalue))

(fn `UpdateHP`
  (params (PlayerNumber :type Integer))
  ;[1 1 1] Do get all the necessary references
  (bind _aspang_hud (cast `/Game/PangBP/Blueprints/GameMode/PangHUD` (`PlayerController.GetHUD` (`GameplayStatics.GetPlayerController` 0)))
    (:`then`
      (bind _asin__game_widget (cast `/Game/PangBP/Blueprints/UI/In-GameWidget` (`/Game/PangBP/Blueprints/GameMode/PangHUD.CurrentWidget` _aspang_hud))
        (:`then`
          (bind _aspang_game_instance_bp (cast `/Game/PangBP/Blueprints/GameMode/PangGameInstance_BP` (`GameplayStatics.GetGameInstance`)))
          (switch `int` PlayerNumber
            (:`Default`
              ;[1 1 1] Set HP images for P1
              (switch `int` (`/Game/PangBP/Blueprints/GameMode/PangGameInstance_BP.PH1Left` _aspang_game_instance_bp) :!label _label
                (:`0`
                  (`Widget.SetVisibility` (`/Game/PangBP/Blueprints/UI/In-GameWidget.Life1` _asin__game_widget) "Hidden")
                  (`Widget.SetVisibility` (`/Game/PangBP/Blueprints/UI/In-GameWidget.Life2` _asin__game_widget) "Hidden" :!label _label_2))
                (:`1`
                  (goto _label_2))
                (:`2`
                  _))
              (`Widget.SetVisibility` (`/Game/PangBP/Blueprints/UI/In-GameWidget.Life3` _asin__game_widget) "Hidden"))
            (:`0`
              (goto _label))
            (:`1`
              ;[1 1 1] Set HP images for P2
              (switch `int` (`/Game/PangBP/Blueprints/GameMode/PangGameInstance_BP.PH2Left` _aspang_game_instance_bp)
                (:`0`
                  (`Widget.SetVisibility` (`/Game/PangBP/Blueprints/UI/In-GameWidget.LifeP21` _asin__game_widget) "Hidden")
                  (`Widget.SetVisibility` (`/Game/PangBP/Blueprints/UI/In-GameWidget.LifeP22` _asin__game_widget) "Hidden" :!label _label_3))
                (:`1`
                  (goto _label_3))
                (:`2`
                  _))
              (`Widget.SetVisibility` (`/Game/PangBP/Blueprints/UI/In-GameWidget.LifeP23` _asin__game_widget) "Hidden"))))
        (:`CastFailed`
          (`KismetSystemLibrary.PrintString` "wrong widget"))))
    (:`CastFailed`
      (`KismetSystemLibrary.PrintString` "Wrong HUD, change to PangHUD"))))

(fn `UpdateTime`
  ;[1 1 1] Check if time is over and if so, trigger the end level evnts
  (bind _aspang_hud (cast `/Game/PangBP/Blueprints/GameMode/PangHUD` (`PlayerController.GetHUD` (`GameplayStatics.GetPlayerController` 0)))
    (:`then`
      (bind _asin__game_widget (cast `/Game/PangBP/Blueprints/UI/In-GameWidget` (`/Game/PangBP/Blueprints/GameMode/PangHUD.CurrentWidget` _aspang_hud)))
      (bind _result (`/Engine/EditorBlueprintResources/StandardMacros.DecrementFloat` (`self.TimeLeft`))
        (:`  `
          (`TextBlock.SetText` (`/Game/PangBP/Blueprints/UI/In-GameWidget.TimeNumber` _asin__game_widget) (`|FormatText` "{Value}" _result))
          (if (<= _result 0.0)
            (set `self.IsEndLevel` true)
            (bind _aspang_game_instance_bp (cast `/Game/PangBP/Blueprints/GameMode/PangGameInstance_BP` (`GameplayStatics.GetGameInstance`)))
            (bind _aspang_hud_2 (cast `/Game/PangBP/Blueprints/GameMode/PangHUD` (`PlayerController.GetHUD` (`GameplayStatics.GetPlayerController` 0))))
            (bind _asin__game_widget_2 (cast `/Game/PangBP/Blueprints/UI/In-GameWidget` (`/Game/PangBP/Blueprints/GameMode/PangHUD.CurrentWidget` _aspang_hud_2)))
            ;;[1 1 1] Trigger the animations
            (if (`/Game/PangBP/Blueprints/GameMode/PangGameInstance_BP.Competitive?` _aspang_game_instance_bp)
              (`/Game/PangBP/Blueprints/UI/In-GameWidget.CompetitiveEndAnim` _asin__game_widget_2)
              (else
                (`/Game/PangBP/Blueprints/UI/In-GameWidget.GameOverAnim` _asin__game_widget_2)))))))
    (:`CastFailed`
      (`KismetSystemLibrary.PrintString` "Wrong HUD, change to PangHUD"))))

(fn `UserConstructionScript`)