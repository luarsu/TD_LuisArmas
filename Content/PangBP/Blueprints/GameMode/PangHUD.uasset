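; PangHUD creates the on-screen UI for a Pang game, choosing the widget by current level name.
; SetUI shows the main menu widget on MainMenuMap, otherwise the in-game widget, storing either as CurrentWidget.
; For gameplay, it has PangGameMode refresh both players' HP and the time, then pauses the game and plays the intro animation.
; If the game instance flags two players, it also spawns player 2 and shows their UI.
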(event `SetUI`
  (bind _returnvalue (`GameplayStatics.GetCurrentLevelName` true))
  (if (`KismetStringLibrary.EqualEqual_StrStr` _returnvalue "MainMenuMap")
    ;[1 1 1] Add Main Menu UI to the game
    (bind _returnvalue_2 (`|CreateWidget` "/Game/PangBP/Blueprints/UI/MainMenuWidget.MainMenuWidget_C"))
    (`UserWidget.AddToViewport` _returnvalue_2 0)
    (set `self.CurrentWidget` _returnvalue_2)
    (else
      ;[1 1 1] Add gameplay UI to the game and prepare everything necessary for it
      (bind _returnvalue_3 (`|CreateWidget` "/Game/PangBP/Blueprints/UI/In-GameWidget.In-GameWidget_C"))
      (`UserWidget.AddToViewport` _returnvalue_3 0)
      (set `self.CurrentWidget` _returnvalue_3)
      (bind _aspang_game_mode (cast `/Game/PangBP/Blueprints/GameMode/PangGameMode` (`GameplayStatics.GetGameMode`))
        (:`then`
          ;;[1 1 1] Make sure HP showed is correct
          (`/Game/PangBP/Blueprints/GameMode/PangGameMode.UpdateHP` _aspang_game_mode 0)
          (`/Game/PangBP/Blueprints/GameMode/PangGameMode.UpdateHP` _aspang_game_mode 1)
          (`/Game/PangBP/Blueprints/GameMode/PangGameMode.SetTime` _aspang_game_mode)
          ;;[1 1 1] Play Initial animation
          (`GameplayStatics.SetGamePaused` true)
          (`/Game/PangBP/Blueprints/UI/In-GameWidget.PlayInitAnim` _returnvalue_3)
          ;;[1 1 1] Spawn player 2 if 2 players mode selected
          (bind _aspang_game_instance_bp (cast `/Game/PangBP/Blueprints/GameMode/PangGameInstance_BP` (`GameplayStatics.GetGameInstance`)))
          (if (`/Game/PangBP/Blueprints/GameMode/PangGameInstance_BP.TwoPlayers?` _aspang_game_instance_bp)
            (`/Game/PangBP/Blueprints/GameMode/PangGameMode.SpawnPlayer2` _aspang_game_mode)
            (`/Game/PangBP/Blueprints/GameMode/PangGameMode.ShowP2UI` _aspang_game_mode)))
        (:`CastFailed`
          (`KismetSystemLibrary.PrintString` "Wrong game mode"))))))

(fn `UserConstructionScript`)