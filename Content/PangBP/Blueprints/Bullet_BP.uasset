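; Bullet_BP is the player's projectile in a Pang-style game, destroying itself on contact and splitting any bubble it strikes.
; Each tick it moves straight up along world Z by Speed, setting its location without sweep.
; The sphere's hit and begin-overlap events both feed CheckCollision, since bubbles register hits while map borders register overlaps.
; A Destroyed flag prevents double handling before it calls Divide on a Bubble_BP and destroys itself.
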(event `self.ReceiveTick`
  (params (DeltaSeconds :type "Float (single-precision)"))
  ;[1 1 1] Move up
  (`self.K2_SetActorLocation` (+ (`self.K2_GetActorLocation`) (`KismetMathLibrary.MakeVector` 0.0 0.0 (`self.Speed`)))))

(event `self.Sphere.OnComponentHit`
  (params (HitComponent :type "PrimitiveComponent Object Reference") (OtherActor :type "Actor Object Reference") (OtherComp :type "PrimitiveComponent Object Reference") (NormalImpulse :type "Vector Structure") (Hit :type "HitResult Structure (by ref)"))
  ;[1 1 1] Check collisions
  ;;[1 1 1] Hit detects the bubbles but not the overlap with the map borthers
  ;;[1 1 1] Created function to aviod duplicated code
  (`self.CheckCollision` OtherActor))

(event `self.Sphere.OnComponentBeginOverlap`
  (params (OverlappedComponent :type "PrimitiveComponent Object Reference") (OtherActor :type "Actor Object Reference") (OtherComp :type "PrimitiveComponent Object Reference") (OtherBodyIndex :type Integer) (bFromSweep :type Boolean) (SweepResult :type "HitResult Structure (by ref)"))
  ;[1 1 1] Check collisions
  ;;[1 1 1] Hit detects the bubbles but not the overlap with the map borthers
  ;;[1 1 1] Created function to aviod duplicated code
  (`self.CheckCollision` OtherActor))

(fn `CheckCollision`
  (params (Actor :type "Actor Object Reference"))
  ;[1 1 1] Make sure that its not called twice when multiple collision events are generated
  (if (not (`self.Destroyed`))
    (set `self.Destroyed` true)
    (bind _asbubble_bp (cast `/Game/PangBP/Blueprints/Bubble_BP` Actor)
      (:`then`
        ;[1 1 1] Call the divide function in the bubble
        (`/Game/PangBP/Blueprints/Bubble_BP.Divide` _asbubble_bp 0))
      (:`CastFailed`
        _))
    (`self.K2_DestroyActor`)))

(fn `UserConstructionScript`)