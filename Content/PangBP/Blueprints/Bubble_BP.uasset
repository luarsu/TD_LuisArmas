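; Bouncing bubble actor for a Pang-style game, launched in a random Y/Z direction by projectile movement and counted in PangGameMode.
; Divide spawns two half-scale bubbles while DivisionsLeft remains, then decrements the game mode count and destroys the actor.
; DisablePhysics freezes it by storing velocity and zeroing gravity until a timer calls EnablePhysics.
; Bubbles split while frozen pass the remaining freeze time to their children.
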(event `self.ReceiveBeginPlay`
  (bind _projectilemovement (`self.ProjectileMovement`))
  ;[1 1 1] Add itself to the bubbles array in the game mode when created
  (bind _aspang_game_mode (cast `/Game/PangBP/Blueprints/GameMode/PangGameMode` (`GameplayStatics.GetGameMode`)))
  (set `/Game/PangBP/Blueprints/GameMode/PangGameMode.NumberOfBubbles` (+ (`/Game/PangBP/Blueprints/GameMode/PangGameMode.NumberOfBubbles` _aspang_game_mode) 1) _aspang_game_mode)
  ;[1 1 1] Randomise initial direction
  (set `MovementComponent.Velocity` (`KismetMathLibrary.MakeVector` 0.0 (`KismetMathLibrary.RandomFloatInRange` -3000.0 3000.0) (`KismetMathLibrary.RandomFloatInRange` 1000.0 3000.0)) _projectilemovement)
  (set `ProjectileMovementComponent.InitialSpeed` 2000.0 _projectilemovement))

(fn `DisablePhysics`
  (params (TimeLeft :type "Float (double-precision)"))
  (bind _projectilemovement (`self.ProjectileMovement`))
  ;[1 1 1] Disable projectile physics and create timer
  ;;[1 1 1] Save the velocity for when physics are back
  (set `self.PreviousVelocity` (`MovementComponent.Velocity` _projectilemovement))
  (set `MovementComponent.Velocity` (0.0 0.0 0.0) _projectilemovement)
  (set `ProjectileMovementComponent.ProjectileGravityScale` 0.0 _projectilemovement)
  (bind _returnvalue (`KismetSystemLibrary.K2_SetTimer` null "EnablePhysics" TimeLeft))
  ;;[1 1 1] Created to pass the value to the new created bubbles if destroyed
  (set `self.IsFrozen` true)
  (set `self.TimerFrozenLeft` _returnvalue))

(fn `Divide`
  (bind _returnvalue (/ (`self.GetActorScale3D`) 2.0))
  (bind _returnvalue_2 (`KismetSystemLibrary.K2_GetTimerRemainingTimeHandle` (`self.TimerFrozenLeft`)))
  (bind _returnvalue_3 (- (`self.DivisionsLeft`) 1))
  ;[1 1 1] Check if there are any divisions left, otherwise destroy
  (if (>= (`self.DivisionsLeft`) 1)
    ;[1 1 1] Create the two new smaller bubbles when main bubble is hit
    (bind _returnvalue_4 (`|SpawnActorFromClass` "Bubble_BP_C" (`KismetMathLibrary.MakeTransform` (+ (`self.K2_GetActorLocation`) (0.0 75.0 0.0)) (struct) _returnvalue) "AdjustIfPossibleButAlwaysSpawn" "OverrideRootScale" null null))
    (set `/Game/PangBP/Blueprints/Bubble_BP.DivisionsLeft` _returnvalue_3 _returnvalue_4)
    (bind _returnvalue_5 (`|SpawnActorFromClass` "Bubble_BP_C" (`KismetMathLibrary.MakeTransform` (+ (`self.K2_GetActorLocation`) (0.0 -75.0 0.0)) (struct) _returnvalue) "AdjustIfPossibleButAlwaysSpawn" "OverrideRootScale" null null))
    (set `/Game/PangBP/Blueprints/Bubble_BP.DivisionsLeft` _returnvalue_3 _returnvalue_5)
    ;[1 1 1] If the hourglass is actie, the new bubbles must be frozen too
    (if (`self.IsFrozen`)
      (`self.DisablePhysics` _returnvalue_5 _returnvalue_2)
      (`self.DisablePhysics` _returnvalue_4 _returnvalue_2)))
  ;[1 1 1] Remove self from bubble game mode list when destroyed
  (bind _aspang_game_mode (cast `/Game/PangBP/Blueprints/GameMode/PangGameMode` (`GameplayStatics.GetGameMode`)))
  (set `/Game/PangBP/Blueprints/GameMode/PangGameMode.NumberOfBubbles` (- (`/Game/PangBP/Blueprints/GameMode/PangGameMode.NumberOfBubbles` _aspang_game_mode) 1) _aspang_game_mode)
  (`self.K2_DestroyActor`))

(fn `EnablePhysics`
  (bind _projectilemovement (`self.ProjectileMovement`))
  ;[1 1 1] Enable physics back
  (set `MovementComponent.Velocity` (`self.PreviousVelocity`) _projectilemovement)
  (set `ProjectileMovementComponent.ProjectileGravityScale` 1.0 _projectilemovement)
  (set `self.IsFrozen` false))

(fn `UserConstructionScript`)