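; Player character for a Pang-style game, with side movement, jumping and weapon-based shooting.
; Player 1's instance also forwards second-player keys to character 1 in two-player mode, working around shared-keyboard limits.
; Shoot spawns capped harpoons, hooks or uncapped bullets by CurrentWeapon; DisableWeapon restores the default and updates the UI.
; Bubble hits consume the invulnerability shield or print "Dead"; the HP-decrement logic is disconnected.
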(event `InputAction|Jump` :overrideparent false
  (params (Key :type "Key Structure"))
  ;[1 1 1] Controls for character 1
  ;;[1 1 1] Jump character 1
  (:`Pressed`
    (`self.Jump` :!label _label))
  (:`Released`
    (`self.StopJumping` :!label _label_2)))

(event `InputAxis|MoveRight` :overrideparent false
  (params (AxisValue :type "Float (single-precision)"))
  ;[1 1 1] Controls for character 1
  ;;[1 1 1] Movement input character 1
  (`self.AddMovementInput` (0.0 -1.0 0.0) AxisValue))

(event `InputTouch`
  (params (Location :type "Vector Structure") (FingerIndex :type "ETouchIndex Enum"))
  ;[1 1 1] Controls for character 1
  ;;[1 1 1] Jump character 1
  (:`Pressed`
    (goto _label))
  (:`Released`
    (goto _label_2)))

(event `InputAction|Shoot`
  (params (Key :type "Key Structure"))
  ;[1 1 1] Controls for character 1
  ;;[1 1 1] Shoot for character 1
  (:`Pressed`
    (`self.Shoot` self)))

(event `InputAxis|MoveRight2`
  (params (AxisValue :type "Float (single-precision)"))
  ;[1 1 1] Input for character 2. As unreal downst allow two players to use the same keyboard, I had to bypass that manually
  ;;[1 1 1] Move Character2
  (bind _aspang_game_mode (cast `/Game/PangBP/Blueprints/GameMode/PangGameMode` (`GameplayStatics.GetGameMode`)))
  (if (`/Game/PangBP/Blueprints/GameMode/PangGameMode.TwoPlayers?` _aspang_game_mode)
    (`self.AddMovementInput` (`GameplayStatics.GetPlayerPawn` 1) (0.0 -1.0 0.0) AxisValue false)))

(event `InputAction|Jump2`
  (params (Key :type "Key Structure"))
  (bind _returnvalue (`GameplayStatics.GetPlayerCharacter` 1))
  ;[1 1 1] Input for character 2. As unreal downst allow two players to use the same keyboard, I had to bypass that manually
  ;;[1 1 1] Jump for character 2
  (:`Pressed`
    (bind _aspang_game_mode (cast `/Game/PangBP/Blueprints/GameMode/PangGameMode` (`GameplayStatics.GetGameMode`)))
    (if (`/Game/PangBP/Blueprints/GameMode/PangGameMode.TwoPlayers?` _aspang_game_mode)
      (`self.Jump` _returnvalue)))
  (:`Released`
    (bind _aspang_game_mode_2 (cast `/Game/PangBP/Blueprints/GameMode/PangGameMode` (`GameplayStatics.GetGameMode`)))
    (if (`/Game/PangBP/Blueprints/GameMode/PangGameMode.TwoPlayers?` _aspang_game_mode_2)
      (`self.StopJumping` _returnvalue))))

(event `InputAction|Shoot2`
  (params (Key :type "Key Structure"))
  ;[1 1 1] Input for character 2. As unreal downst allow two players to use the same keyboard, I had to bypass that manually
  ;;[1 1 1] Shoot for character 2
  (:`Pressed`
    (bind _aspang_game_mode (cast `/Game/PangBP/Blueprints/GameMode/PangGameMode` (`GameplayStatics.GetGameMode`)))
    (if (`/Game/PangBP/Blueprints/GameMode/PangGameMode.TwoPlayers?` _aspang_game_mode)
      (bind _aspang_character_bp (cast `/Game/PangBP/Blueprints/PangCharacter_BP` (`GameplayStatics.GetPlayerCharacter` 1)))
      (`self.Shoot` _aspang_character_bp _aspang_character_bp))))

(event `self.CapsuleComponent.OnComponentHit`
  (params (HitComponent :type "PrimitiveComponent Object Reference") (OtherActor :type "Actor Object Reference") (OtherComp :type "PrimitiveComponent Object Reference") (NormalImpulse :type "Vector Structure") (Hit :type "HitResult Structure (by ref)"))
  ;[1 1 1] Check collisions with the bubbles and update hp when hit
  (cast `/Game/PangBP/Blueprints/Bubble_BP` OtherActor)
  (if (`self.Is invulnerable`)
    (set `self.Is invulnerable` false)
    (`SceneComponent.SetVisibility` (`self.Sphere`) false false)
    (else
      (`KismetSystemLibrary.PrintString` "Dead")
      (bind _aspang_game_mode (cast `/Game/PangBP/Blueprints/GameMode/PangGameMode` (`GameplayStatics.GetGameMode`))))))

(fn `DisableWeapon`
  ;[1 1 1] Function called by timer, just disabled by time
  (bind _output_get (set `self.CurrentWeapon` 0))
  (bind _aspang_game_mode (cast `/Game/PangBP/Blueprints/GameMode/PangGameMode` (`GameplayStatics.GetGameMode`))
    (:`then`
      (`/Game/PangBP/Blueprints/GameMode/PangGameMode.ChangePlayerWeaponUI` _aspang_game_mode (`self.PlayerID`) _output_get))
    (:`CastFailed`
      (`KismetSystemLibrary.PrintString` "Wrong game mode"))))

(fn `Shoot`
  (params (CharacterShooting :type "/Game/PangBP/Blueprints/PangCharacter_BP Object Reference"))
  (bind _currentweapon (`/Game/PangBP/Blueprints/PangCharacter_BP.CurrentWeapon` CharacterShooting))
  (bind _numberhooks (`/Game/PangBP/Blueprints/PangCharacter_BP.NumberHooks` CharacterShooting))
  (bind _returnvalue (`KismetMathLibrary.MakeTransform` (`KismetMathLibrary.MakeVector` (.x (`self.K2_GetActorLocation` CharacterShooting)) (.y (`self.K2_GetActorLocation` CharacterShooting)) (`self.ShootHeight`)) (struct) (`self.BulletScale`)))
  ;[1 1 1] Select the appropiate projectile to create based on the powerups
  (switch `int` _currentweapon
    (:`0`
      ;[1 1 1] In the original game you can only shoot one at a time (unless you have boosters)
      (if (< _numberhooks 1) :!label _label
        (bind _returnvalue_2 (`|SpawnActorFromClass` "/Game/PangBP/Blueprints/Harpoon_BP.Harpoon_BP_C" _returnvalue "AlwaysSpawn" "OverrideRootScale" null null :!label _label_2))
        ;[1 1 1] Set reference so they know which player created it
        (set `/Game/PangBP/Blueprints/Harpoon_BP.CreatorCharacter` CharacterShooting _returnvalue_2)
        ;[1 1 1] keep track of number of hooks alive at the same time
        (`/Engine/EditorBlueprintResources/StandardMacros.IncrementInt` _numberhooks
          (:`  `
            ;[1 1 1] Set the created object as a hook if the power up is activated
            (switch `int` _currentweapon
              (:`1`
                (set `/Game/PangBP/Blueprints/Harpoon_BP.Hook` true _returnvalue_2)))))))
    (:`1`
      (goto _label))
    (:`2`
      ;[1 1 1] If the power up of double hooks is active, check this condition instead of the other
      (if (< _numberhooks 2)
        (goto _label_2)))
    (:`3`
      ;[1 1 1] Spawn bullet
      (bind _returnvalue_3 (`|SpawnActorFromClass` "/Game/PangBP/Blueprints/Bullet_BP.Bullet_BP_C" _returnvalue "AlwaysSpawn" "OverrideRootScale" null null))
      (set `/Game/PangBP/Blueprints/Bullet_BP.CreatorCharacter` CharacterShooting _returnvalue_3))))

(fn `UserConstructionScript`)