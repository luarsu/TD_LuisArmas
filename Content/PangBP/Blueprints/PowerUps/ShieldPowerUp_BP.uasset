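; Shield power-up pickup for the Pang game that protects the player character.
; On BeginPlay it binds HookPowerUp to a component picked-up event.
; When fired, the handler casts the picking actor to PangCharacter_BP, sets IsInvulnerable and shows the character's Sphere component as the shield.
; This graph sets no duration and never switches the shield off.
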(event `self.ReceiveBeginPlay`
  (`parent.ReceiveBeginPlay`)
  (add `self.OnComponentPickedUp` (delegate `HookPowerUp`)))

(event `HookPowerUp` :!signature `self.OnComponentPickedUp`
  (params (ActorReference :type "Actor Object Reference"))
  ;[1 1 1] Set shield to visible and booblean variable to true
  (bind _aspang_character_bp (cast `/Game/PangBP/Blueprints/PangCharacter_BP` ActorReference))
  (set `/Game/PangBP/Blueprints/PangCharacter_BP.Is invulnerable` true _aspang_character_bp)
  (`SceneComponent.SetVisibility` (`/Game/PangBP/Blueprints/PangCharacter_BP.Sphere` _aspang_character_bp) true false))

(fn `UserConstructionScript`
  (`parent.UserConstructionScript`))