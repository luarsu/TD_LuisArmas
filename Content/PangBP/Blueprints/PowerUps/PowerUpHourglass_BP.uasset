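; Hourglass power-up pickup that freezes bubbles by temporarily disabling their physics.
; On BeginPlay it binds to its component's picked-up event and reacts only when the collector is a PangCharacter_BP.
; It then calls DisablePhysics on every Bubble_BP with a fixed duration.
; DestroyActor sits inside that loop, so the pickup removes itself only if at least one bubble exists.
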(event `self.ReceiveBeginPlay`
  (`parent.ReceiveBeginPlay`)
  (add `self.OnComponentPickedUp` (delegate `HookPowerUp`)))

(event `HookPowerUp` :!signature `self.OnComponentPickedUp`
  (params (ActorReference :type "Actor Object Reference"))
  ;[1 1 1] Get all the bubbles, disable physics and set a timer for end of the hourglass effect
  (cast `/Game/PangBP/Blueprints/PangCharacter_BP` ActorReference)
  (bind _outactors (`GameplayStatics.GetAllActorsOfClass` "/Game/PangBP/Blueprints/Bubble_BP.Bubble_BP_C"))
  (for _array_element _outactors
    (`/Game/PangBP/Blueprints/Bubble_BP.DisablePhysics` _array_element 7.0)
    (`self.K2_DestroyActor`)))

(fn `UserConstructionScript`
  (`parent.UserConstructionScript`))