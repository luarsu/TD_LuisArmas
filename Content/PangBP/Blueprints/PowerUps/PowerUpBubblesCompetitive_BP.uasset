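; Competitive bubbles power-up pickup that switches the collecting Pang character to the bubble weapon.
; On BeginPlay it binds to the component's picked-up event, then sets the character's current weapon and refills its bubble count.
; It updates that player's weapon UI through PangGameMode and destroys itself, or prints an error if the game mode is wrong.
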(event `self.ReceiveBeginPlay`
  (`parent.ReceiveBeginPlay`)
  (add `self.OnComponentPickedUp` (delegate `HookPowerUp`)))

(event `HookPowerUp` :!signature `self.OnComponentPickedUp`
  (params (ActorReference :type "Actor Object Reference"))
  ;[1 1 1] Set the player weapon to the gun, and a timer to disable it after some time
  (bind _aspang_character_bp (cast `/Game/PangBP/Blueprints/PangCharacter_BP` ActorReference))
  (bind _output_get (set `/Game/PangBP/Blueprints/PangCharacter_BP.CurrentWeapon` 4 _aspang_character_bp))
  (set `/Game/PangBP/Blueprints/PangCharacter_BP.BubblesLeft` 3 _aspang_character_bp)
  (bind _aspang_game_mode (cast `/Game/PangBP/Blueprints/GameMode/PangGameMode` (`GameplayStatics.GetGameMode`))
    (:`then`
      (`/Game/PangBP/Blueprints/GameMode/PangGameMode.ChangePlayerWeaponUI` _aspang_game_mode (`/Game/PangBP/Blueprints/PangCharacter_BP.PlayerID` _aspang_character_bp) _output_get)
      (`self.K2_DestroyActor`))
    (:`CastFailed`
      (`KismetSystemLibrary.PrintString` "Wrong game mode"))))

(fn `UserConstructionScript`
  (`parent.UserConstructionScript`))