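; Score power-up pickup that awards extra points to the Pang character that collects it.
; On BeginPlay it binds its handler to the OnComponentPickedUp event.
; When triggered, the handler passes ScoreToAdd and the character's PlayerID to PangGameMode's ScoreAnimation, then destroys the actor.
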(event `self.ReceiveBeginPlay`
  (`parent.ReceiveBeginPlay`)
  (add `self.OnComponentPickedUp` (delegate `HookPowerUp`)))

(event `HookPowerUp` :!signature `self.OnComponentPickedUp`
  (params (ActorReference :type "Actor Object Reference"))
  ;[1 1 1] Adds extra score for the player
  (bind _aspang_character_bp (cast `/Game/PangBP/Blueprints/PangCharacter_BP` ActorReference))
  (bind _aspang_game_mode (cast `/Game/PangBP/Blueprints/GameMode/PangGameMode` (`GameplayStatics.GetGameMode`)))
  (`/Game/PangBP/Blueprints/GameMode/PangGameMode.ScoreAnimation` _aspang_game_mode (`self.ScoreToAdd`) (`/Game/PangBP/Blueprints/PangCharacter_BP.PlayerID` _aspang_character_bp))
  (`self.K2_DestroyActor`))

(fn `UserConstructionScript`
  (`parent.UserConstructionScript`))