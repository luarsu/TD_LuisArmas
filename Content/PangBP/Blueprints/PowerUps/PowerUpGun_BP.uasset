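; Gun power-up pickup for a Pang-style game that temporarily arms the collecting player with the gun weapon.
; On BeginPlay it binds to the component picked-up event, then casts the collector to PangCharacter_BP and proceeds only if no other special weapon is active.
; It sets the weapon, starts a named timer for the character's DisableWeapon, updates the weapon UI through PangGameMode and destroys itself.
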(event `self.ReceiveBeginPlay`
  (`parent.ReceiveBeginPlay`)
  (add `self.OnComponentPickedUp` (delegate `HookPowerUp`)))

(event `HookPowerUp` :!signature `self.OnComponentPickedUp`
  (params (ActorReference :type "Actor Object Reference"))
  ;[1 1 1] Set the player weapon to the gun, and a timer to disable it after some time
  (bind _aspang_character_bp (cast `/Game/PangBP/Blueprints/PangCharacter_BP` ActorReference))
  ;;[1 1 1] Only get power up if no other buf weapon is on
  (if (not (!= (`/Game/PangBP/Blueprints/PangCharacter_BP.CurrentWeapon` _aspang_character_bp) 0))
    (bind _output_get (set `/Game/PangBP/Blueprints/PangCharacter_BP.CurrentWeapon` 3 _aspang_character_bp))
    (`KismetSystemLibrary.K2_SetTimer` _aspang_character_bp "DisableWeapon" (`self.PowerUpTime`))
    (bind _aspang_game_mode (cast `/Game/PangBP/Blueprints/GameMode/PangGameMode` (`GameplayStatics.GetGameMode`))
      (:`then`
        (`/Game/PangBP/Blueprints/GameMode/PangGameMode.ChangePlayerWeaponUI` _aspang_game_mode (`/Game/PangBP/Blueprints/PangCharacter_BP.PlayerID` _aspang_character_bp) _output_get)
        (`self.K2_DestroyActor`))
      (:`CastFailed`
        (`KismetSystemLibrary.PrintString` "Wrong game mode")))))

(fn `UserConstructionScript`
  (`parent.UserConstructionScript`))