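; Gun power-up pickup that gives the Pang character a temporary weapon.
; On BeginPlay it binds HookPowerUp to the pickup event; the handler casts the collector to PangCharacter_BP and sets its CurrentWeapon to 3.
; A timer set by function name then calls DisableWeapon on the character after PowerUpTime.
; The handler name and comment refer to a hook, although the asset is named Gun.
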(event `self.ReceiveBeginPlay`
  (`parent.ReceiveBeginPlay`)
  (add `self.OnComponentPickedUp` (delegate `HookPowerUp`)))

(event `HookPowerUp` :!signature `self.OnComponentPickedUp`
  (params (ActorReference :type "Actor Object Reference"))
  ;[1 1 1] Set the player weapon to the hook, and a timer to disable it after some time
  (bind _aspang_character_bp (cast `/Game/PangBP/Blueprints/PangCharacter_BP` ActorReference))
  (set `/Game/PangBP/Blueprints/PangCharacter_BP.CurrentWeapon` 3 _aspang_character_bp)
  (`KismetSystemLibrary.K2_SetTimer` _aspang_character_bp "DisableWeapon" (`self.PowerUpTime`)))

(fn `UserConstructionScript`
  (`parent.UserConstructionScript`))