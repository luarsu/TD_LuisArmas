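; Harpoon projectile for a Pang-style game that climbs each tick, trailing a cable anchored near floor height, and splits bubbles it hits.
; Cone and box collision events feed CheckCollision, guarded against duplicate hits.
; A hit normally decrements the player's hook count, re-enables shooting and destroys the arrow.
; In Hook mode, hitting anything except bubbles or destructible blocks stops it, still collidable, until a timer re-enables shooting and destroys it.
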(event `self.ReceiveTick`
  (params (DeltaSeconds :type "Float (single-precision)"))
  ;[1 1 1] Move the arrow up
  ;;[1 1 1] Condition for hook power up weapon
  (if (not (`self.StopMoving`))
    (`self.K2_SetActorLocation` (+ (`self.K2_GetActorLocation`) (`KismetMathLibrary.MakeVector` 0.0 0.0 (`self.Speed`))))
    ;[1 1 1] Avoid trying to set this when pending to destroy
    (if (not (`self.Destroyed`))
      ;[1 1 1] Update the cable anchor position
      (bind _output_get (set `self.CableRootPosition` (`KismetMathLibrary.InverseTransformLocation` (`self.GetTransform`) (`KismetMathLibrary.MakeVector` (.x (`self.K2_GetActorLocation`)) (.y (`self.K2_GetActorLocation`)) 40.0))))
      (set `CableComponent.EndLocation` _output_get (`self.Cable`)))))

(event `self.Cone.OnComponentHit`
  (params (HitComponent :type "PrimitiveComponent Object Reference") (OtherActor :type "Actor Object Reference") (OtherComp :type "PrimitiveComponent Object Reference") (NormalImpulse :type "Vector Structure") (Hit :type "HitResult Structure (by ref)"))
  ;[1 1 1] Check the collisions
  ;;[1 1 1] Hit detects the bubbles but not the overlap with the map borthers
  ;;[1 1 1] Created function to aviod duplicated code
  (`self.Check Collision` OtherActor))

(event `self.Cone.OnComponentBeginOverlap`
  (params (OverlappedComponent :type "PrimitiveComponent Object Reference") (OtherActor :type "Actor Object Reference") (OtherComp :type "PrimitiveComponent Object Reference") (OtherBodyIndex :type Integer) (bFromSweep :type Boolean) (SweepResult :type "HitResult Structure (by ref)"))
  ;[1 1 1] Check the collisions
  ;;[1 1 1] Hit detects the bubbles but not the overlap with the map borthers
  ;;[1 1 1] Created function to aviod duplicated code
  (`self.Check Collision` OtherActor))

(event `self.Box.OnComponentHit`
  (params (HitComponent :type "PrimitiveComponent Object Reference") (OtherActor :type "Actor Object Reference") (OtherComp :type "PrimitiveComponent Object Reference") (NormalImpulse :type "Vector Structure") (Hit :type "HitResult Structure (by ref)"))
  ;[1 1 1] Check the collisions
  ;;[1 1 1] Created function to aviod duplicated code
  (`self.Check Collision` OtherActor))

(fn `Check Collision`
  (params (Actor :type "Actor Object Reference"))
  ;[1 1 1] Chechks if it has hit the bubble, otherwise it just dissapears
  ;;[1 1 1] Make sure that its not called twice when multiple collision events are generated
  (if (not (`self.Destroyed`))
    (set `self.Destroyed` true)
    (bind _asbubble_bp (cast `/Game/PangBP/Blueprints/Bubble_BP` Actor)
      (:`then`
        ;;[1 1 1] Call the divide function in the bubble
        (`/Game/PangBP/Blueprints/Bubble_BP.Divide` _asbubble_bp)
        (bind _aspang_character_bp (cast `/Game/PangBP/Blueprints/PangCharacter_BP` (`GameplayStatics.GetPlayerCharacter` 0) :!label _label))
        (`/Engine/EditorBlueprintResources/StandardMacros.DecrementInt` (`/Game/PangBP/Blueprints/PangCharacter_BP.NumberHooks` _aspang_character_bp)
          (:`  `
            ;[1 1 1] Restore shooting for player once destroyed
            (set `/Game/PangBP/Blueprints/PangCharacter_BP.CanShoot` true _aspang_character_bp)
            (`self.K2_DestroyActor`))))
      (:`CastFailed`
        ;;[1 1 1] Condition to check onyl when weapon is hook powerup
        (if (`self.Hook`)
          ;[1 1 1] check that is not a destructible block
          (cast `/Game/PangBP/Blueprints/DestructableBlock_BP` Actor
            (:`then`
              (goto _label))
            (:`CastFailed`
              ;[1 1 1] If it's a hook, then just stop moving and set timer to autodestroy
              (set `self.StopMoving` true)
              (`KismetSystemLibrary.K2_SetTimer` self "DestroySelf" 5.0)
              (set `self.Destroyed` false)))
          (else
            (goto _label)))))))

(fn `DestroySelf`
  ;[1 1 1] Just a function to destroy itself after some time (hook powerup)
  (bind _aspang_character_bp (cast `/Game/PangBP/Blueprints/PangCharacter_BP` (`GameplayStatics.GetPlayerCharacter` 0)))
  (set `/Game/PangBP/Blueprints/PangCharacter_BP.CanShoot` true _aspang_character_bp)
  (`self.K2_DestroyActor`))

(fn `UserConstructionScript`)